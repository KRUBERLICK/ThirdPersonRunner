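; Right-corner floor tile actor for the runner game, where the player character turns or dies against the walls.
; Overlapping the TurnZone component sets CanTurn on the RG_Character.
; Hitting either of the two wall components calls Death on that character.
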(event `self.TurnZone.OnComponentBeginOverlap`
  (params (OverlappedComponent :type "PrimitiveComponent Object Reference") (OtherActor :type "Actor Object Reference") (OtherComp :type "PrimitiveComponent Object Reference") (OtherBodyIndex :type Integer) (bFromSweep :type Boolean) (SweepResult :type "HitResult Structure (by ref)"))
  (bind _asrg_character (cast `/Game/RunnerGame/GameBP/RG_Character` OtherActor))
  (set `/Game/RunnerGame/GameBP/RG_Character.CanTurn` true _asrg_character))

(event `self.Wall.OnComponentHit`
  (params (HitComponent :type "PrimitiveComponent Object Reference") (OtherActor :type "Actor Object Reference") (OtherComp :type "PrimitiveComponent Object Reference") (NormalImpulse :type "Vector Structure") (Hit :type "HitResult Structure (by ref)"))
  (bind _asrg_character (cast `/Game/RunnerGame/GameBP/RG_Character` OtherActor))
  (`/Game/RunnerGame/GameBP/RG_Character.Death` _asrg_character))

(event `self.Wall2.OnComponentHit`
  (params (HitComponent :type "PrimitiveComponent Object Reference") (OtherActor :type "Actor Object Reference") (OtherComp :type "PrimitiveComponent Object Reference") (NormalImpulse :type "Vector Structure") (Hit :type "HitResult Structure (by ref)"))
  (bind _asrg_character (cast `/Game/RunnerGame/GameBP/RG_Character` OtherActor))
  (`/Game/RunnerGame/GameBP/RG_Character.Death` _asrg_character))

(fn `UserConstructionScript`)